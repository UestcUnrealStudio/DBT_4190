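; Lobby game mode that tracks connected players and launches the match from the lobby.
; On login, the server stores each controller, reads the server name and player limit from GameInfoInstance, and initializes that PC_Lobby's menu.
; EveryoneUpdate rebuilds the player settings list and pushes it, with player counts, to every controller; logout removes the leaver and refreshes.
; LanuchGame uses a servertravel console command to move to PlayMap.
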(event `self.K2_PostLogin`
  (params (NewPlayer :type "PlayerController Object Reference"))
  (`/Engine/EditorBlueprintResources/ActorMacros.Switch Has Authority`
    (:`Authority`
      (`KismetArrayLibrary.Array_Add` (`self.AllPlayerControllers`) NewPlayer)
      (bind _asgame_info_instance (cast `/Game/BP/AllLevels/GameInfoInstance` (`GameplayStatics.GetGameInstance`)))
      (set `self.ServerName` (`/Game/BP/AllLevels/GameInfoInstance.ServerName` _asgame_info_instance))
      (set `self.MaxPlayer` (`/Game/BP/AllLevels/GameInfoInstance.ServerMaxPlayer` _asgame_info_instance))
      (bind _aspc_lobby (cast `/Game/BP/Lobby/PC_Lobby` NewPlayer))
      (`/Game/BP/Lobby/PC_Lobby.InitialSetup` _aspc_lobby)
      (`/Game/BP/Lobby/PC_Lobby.SetupLobbyMenu` _aspc_lobby (`self.ServerName`)))))

(event `EveryoneUpdate`
  (bind _allplayercontrollers (`self.AllPlayerControllers`))
  ;[1 1 1] 更新Lobby内一切信息
  (bind _output_get (set `self.CurrentPlayers` (`KismetArrayLibrary.Array_Length` (`self.AllPlayerControllers`))))
  (if (> _output_get 0)
    (`KismetArrayLibrary.Array_Clear` (`self.ConnectedPlayers`))
    (for _array_element _allplayercontrollers
      (bind _aspc_lobby (cast `/Game/BP/Lobby/PC_Lobby` _array_element))
      (`KismetArrayLibrary.Array_Add` (`self.ConnectedPlayers`) (`/Game/BP/Lobby/PC_Lobby.PlayerSettings` _aspc_lobby))
      (`/Game/BP/Lobby/PC_Lobby.UpdatePlayerNumber` _aspc_lobby (`self.CurrentPlayers`) (`self.MaxPlayer`)))
    (for _array_element_2 _allplayercontrollers
      (bind _aspc_lobby_2 (cast `/Game/BP/Lobby/PC_Lobby` _array_element_2))
      (`/Game/BP/Lobby/PC_Lobby.AddPlayerInfo` _aspc_lobby_2 (`self.ConnectedPlayers`)))))

(event `self.K2_OnLogout`
  (params (ExitingController :type "Controller Object Reference"))
  ;[1 1 1] 有人退出，更新Lobby
  (for (_array_element _array_index) (`self.AllPlayerControllers`)
    (if (== ExitingController _array_element)
      (break)))
  (cast `/Game/BP/Lobby/PC_Lobby` ExitingController)
  (`KismetArrayLibrary.Array_Remove` (`self.AllPlayerControllers`) _array_index)
  (`KismetArrayLibrary.Array_Remove` (`self.ConnectedPlayers`) _array_index)
  (`self.EveryoneUpdate`))

(event `LanuchGame`
  (`KismetSystemLibrary.ExecuteConsoleCommand` "servertravel /Game/Maps/PlayMap" (`GameplayStatics.GetPlayerController` 0)))

(fn `UserConstructionScript`)
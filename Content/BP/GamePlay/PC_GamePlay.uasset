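; PC_GamePlay is the gameplay player controller that gets each player spawned with their saved character and team.
; On BeginPlay, the local controller clears widgets, loads PlayerSettings from the PlayerSettingsSave slot and passes them to PassPlayerInfoToServer.
; That event stores the settings and asks GM_GamePlay to spawn the player with the chosen character and team.
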(event `self.ReceiveBeginPlay`
  (if (`self.IsLocalController`)
    (`WidgetLayoutLibrary.RemoveAllWidgets`)
    (`self.LoadGame`)
    (`self.PassPlayerInfoToServer` (`self.PlayerSettings`))))

(event `PassPlayerInfoToServer`
  (params (PlayerSettingsInfo :type "/Game/BP/AllLevels/PlayerInfo Structure"))
  (bind _output_get (set `self.PlayerSettings` PlayerSettingsInfo))
  (bind _asgm_game_play (cast `/Game/BP/GamePlay/GM_GamePlay` (`GameplayStatics.GetGameMode`)))
  (bind (_myplayername _myplayeravatarimage _myplayercharactr _team) (break `/Game/BP/AllLevels/PlayerInfo` _output_get))
  (`/Game/BP/GamePlay/GM_GamePlay.SpawnPlayer` _asgm_game_play self _myplayercharactr _team))

(fn `LoadGame`
  (bind _returnvalue (`GameplayStatics.LoadGameFromSlot` (`self.PlayerSettingsSave`)))
  (bind _asplayer_save_game (cast `/Game/BP/AllLevels/PlayerSaveGame` _returnvalue))
  (set `self.PlayerSettings` (`/Game/BP/AllLevels/PlayerSaveGame.PlayerInfo` _asplayer_save_game)))

(fn `UserConstructionScript`)
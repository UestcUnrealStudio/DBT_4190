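; Lobby player controller that manages a player's saved settings, lobby menu and session exit.
; Setup restores name and avatar from a save slot with status "Not Ready"; character or team swaps save, and both paths notify GM_Lobby to update everyone.
; UI events create the menu and loading screen, show player count, rebuild the list ordered by team and refresh character button availability.
; EndPlay destroys the session; being kicked also opens MainMenu.
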(event `InitialSetup`
  (`self.SaveGameCheck`)
  (`self.CallUpdate` (`self.PlayerSettings`)))

(event `CallUpdate`
  (params (PlayerInfo :type "/Game/BP/AllLevels/PlayerInfo Structure"))
  (set `self.PlayerSettings` PlayerInfo)
  (bind _asgm_lobby (cast `/Game/BP/Lobby/GM_Lobby` (`GameplayStatics.GetGameMode`)))
  (`/Game/BP/Lobby/GM_Lobby.EveryoneUpdate` _asgm_lobby))

(event `SetupLobbyMenu`
  (params (ServerName :type Text) (MaxPlayer :type Integer))
  ;[1 1 1] 显示大厅菜单
  (set `self.bShowMouseCursor` true)
  (bind _returnvalue (`|CreateWidget` "/Game/UI/Lobby/LobbyMenu.LobbyMenu_C" null ServerName MaxPlayer))
  (bind _output_get (set `self.LobbyMenuWB` _returnvalue))
  (`UserWidget.AddToViewport` _returnvalue 0)
  (`/Game/UI/Lobby/LobbyMenu.InitializeCharacter` _output_get))

(event `ShowLoadingScreen`
  (`Widget.RemoveFromParent` (`self.LobbyMenuWB`))
  (bind _returnvalue (`|CreateWidget` "/Game/UI/AllLevels/LoadingScreen.LoadingScreen_C" self))
  (`UserWidget.AddToViewport` _returnvalue 0))

(event `SwapCharacter`
  (params (ChoosedCharacter :type "Character Class Reference") (TeamName :type Text))
  (bind _playersettings (`self.PlayerSettings`))
  (if (`KismetSystemLibrary.IsValidClass` ChoosedCharacter)
    (setmembers `/Game/BP/AllLevels/PlayerInfo` :`StructRef` _playersettings :`MyPlayerCharacter` ChoosedCharacter)
    (else
      (setmembers `/Game/BP/AllLevels/PlayerInfo` :`StructRef` _playersettings :`MyPlayerCharacter` null :`Team` TeamName)))
  (`self.SaveGme`)
  (`self.CallUpdate` (`self.PlayerSettings`)))

(event `UpdatePlayerNumber`
  (params (CurrentPlayers :type Integer) (MaxPlayer :type Integer))
  (bind _lobbymenuwb (`self.LobbyMenuWB`))
  (`/Engine/EditorBlueprintResources/StandardMacros.IsValid` _lobbymenuwb
    (:`Is Valid`
      (set `/Game/UI/Lobby/LobbyMenu.PlayerDisplay` (`|FormatText` "{CurrentPlayers}\\{MaxPlayer}" CurrentPlayers MaxPlayer) _lobbymenuwb))))

(event `AddPlayerInfo`
  (params (ConnectPlayersInfo :type "Array of /Game/BP/AllLevels/PlayerInfo Structure") (TeamNumber :type Integer))
  (bind _lobbymenuwb (`self.LobbyMenuWB`))
  (bind _lobbymenuwb_2 (`self.LobbyMenuWB`))
  ;[1 1 1] 更新PlayerList
  (set `self.AllConnectedPlayers` ConnectPlayersInfo)
  (`/Engine/EditorBlueprintResources/StandardMacros.IsValid` _lobbymenuwb
    (:`Is Valid`
      (`/Game/UI/Lobby/LobbyMenu.ClearPlayerList` _lobbymenuwb)
      (for _index (range 1 (+ TeamNumber 1))
        (for _array_element (`self.AllConnectedPlayers`)
          (if (`KismetTextLibrary.EqualEqual_TextText` (`.Team_19_666F2A414731454F6E5C2A9EC59DE8FC` (break `/Game/BP/AllLevels/PlayerInfo` _array_element)) (`KismetTextLibrary.Conv_IntToText` _index))
            (`/Game/UI/Lobby/LobbyMenu.UpdatePlayerWindow` _lobbymenuwb_2 _array_element)
            (`/Game/UI/Lobby/CharacterSelectMenu.CheckButtonAvailable` (`/Game/UI/Lobby/LobbyMenu.CharacterSelectMenu` _lobbymenuwb_2) (`self.AllConnectedPlayers`))))))))

(event `self.ReceiveEndPlay`
  (params (EndPlayReason :type "EEndPlayReason Enum" :default "Destroyed"))
  (`DestroySessionCallbackProxy.DestroySession` self :!label _label))

(event `Kicked`
  (`GameplayStatics.OpenLevel` "MainMenu")
  (goto _label))

(fn `LoadGame`
  (bind _returnvalue (`GameplayStatics.LoadGameFromSlot` (`self.PlayerSettingsSave`)))
  (bind _asplayer_save_game (cast `/Game/BP/AllLevels/PlayerSaveGame` _returnvalue))
  (bind (_myplayername _myplayeravatarimage) (break `/Game/BP/AllLevels/PlayerInfo` (`/Game/BP/AllLevels/PlayerSaveGame.PlayerInfo` _asplayer_save_game)))
  (setmembers `/Game/BP/AllLevels/PlayerInfo` :`StructRef` (`self.PlayerSettings`) :`MyPlayerName` _myplayername :`MyPlayerAvatarImage` _myplayeravatarimage :`MyPlayrReadyStatus` "Not Ready"))

(fn `SaveGameCheck`
  (bind _returnvalue (`GameplayStatics.DoesSaveGameExist` (`self.PlayerSettingsSave`)))
  (if _returnvalue
    (`self.LoadGame`)
    (`self.SaveGme`)
    (else
      (`self.SaveGme`))))

(fn `SaveGme`
  (bind _playersavegameref (`self.PlayerSaveGameRef`))
  (`/Engine/EditorBlueprintResources/StandardMacros.IsValid` (`self.PlayerSaveGameRef`)
    (:`Is Valid`
      _)
    (:`Is Not Valid`
      (bind _returnvalue (`GameplayStatics.CreateSaveGameObject` "/Game/BP/AllLevels/PlayerSaveGame.PlayerSaveGame_C"))
      (set `self.PlayerSaveGameRef` _returnvalue)))
  (set `/Game/BP/AllLevels/PlayerSaveGame.PlayerInfo` (`self.PlayerSettings`) _playersavegameref)
  (`GameplayStatics.SaveGameToSlot` _playersavegameref (`self.PlayerSettingsSave`)))

(fn `UserConstructionScript`)
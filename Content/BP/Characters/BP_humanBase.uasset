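; Base human character Blueprint that provides movement, look and firing actions as custom events.
; Move and look events pass caller-supplied values straight to movement and controller pitch/yaw input.
; Fire spawns a half-scale BP_BulletBase at GunPos, aimed along the camera's rotation with a fixed upward pitch offset.
; CustomJump is an empty stub, and no input bindings or per-frame logic live here.
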(event `MoveForWard`
  (params (WorldDirection :type "Vector Structure") (Value :type "Float (double-precision)"))
  ;[1 1 1] PlayerMovement
  (`self.AddMovementInput` WorldDirection Value))

(event `MoveRight`
  (params (WorldDirection :type "Vector Structure") (Value :type "Float (double-precision)"))
  ;[1 1 1] PlayerMovement
  (`self.AddMovementInput` WorldDirection Value))

(event `LookUp`
  (params (Value :type "Float (double-precision)"))
  (`self.AddControllerPitchInput` Value))

(event `Turn`
  (params (Value :type "Float (double-precision)"))
  (`self.AddControllerYawInput` Value))

(event `Fire`
  (bind _returnvalue (`SceneComponent.K2_GetComponentLocation` (`self.GunPos`)))
  (bind (_returnvalue_roll _returnvalue_pitch _returnvalue_yaw) (`KismetMathLibrary.BreakRotator` (`SceneComponent.K2_GetComponentRotation` (`self.Camera`))))
  (`|SpawnActorFromClass` "/Game/BP/Characters/Bullet/BP_BulletBase.BP_BulletBase_C" (`KismetMathLibrary.MakeTransform` _returnvalue (`KismetMathLibrary.FindLookAtRotation` _returnvalue (+ _returnvalue (* (`KismetMathLibrary.GetForwardVector` (`KismetMathLibrary.MakeRotator` _returnvalue_roll (+ _returnvalue_pitch 10.0) _returnvalue_yaw)) 100.0))) (0.5 0.5 0.5)) "Undefined" "OverrideRootScale" null null))

(fn `CustomJump`)

(fn `UserConstructionScript`)
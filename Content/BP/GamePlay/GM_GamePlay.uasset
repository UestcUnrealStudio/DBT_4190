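; Gameplay game mode that spawns team characters and tracks player controllers in a multiplayer session.
; SpawnPlayer spawns the given character at the first PlayerStart found for TeamA or the second for TeamB, then possesses it.
; If the controller already has a pawn, DestroyActor targets the game mode itself.
; Controller swaps add to AllPlayerControllers; logout asks GameInfoInstance to destroy that player's session.
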(event `self.ReceiveBeginPlay`)

(event `self.K2_OnLogout`
  (params (ExitingController :type "Controller Object Reference"))
  (bind _aspc_game_play (cast `/Game/BP/GamePlay/PC_GamePlay` ExitingController))
  (`/Game/BP/AllLevels/GameInfoInstance.DestroySessionCaller` (cast `/Game/BP/AllLevels/GameInfoInstance` (`GameplayStatics.GetGameInstance`) :!pure true) _aspc_game_play))

(event `self.K2_OnSwapPlayerControllers`
  (params (OldPC :type "PlayerController Object Reference") (NewPC :type "PlayerController Object Reference"))
  (bind _aspc_game_play (cast `/Game/BP/GamePlay/PC_GamePlay` NewPC))
  (`KismetArrayLibrary.Array_Add` (`self.AllPlayerControllers`) _aspc_game_play))

(event `SpawnPlayer`
  (params (PlayerController :type "PlayerController Object Reference") (Character :type "Character Class Reference") (Team :type Text))
  (`KismetSystemLibrary.PrintString` (`KismetSystemLibrary.GetClassDisplayName` Character))
  (`/Engine/EditorBlueprintResources/StandardMacros.IsValid` (`Controller.K2_GetPawn` PlayerController)
    (:`Is Valid`
      (`self.K2_DestroyActor`))
    (:`Is Not Valid`
      _))
  (bind _outactors (`GameplayStatics.GetAllActorsOfClass` "/Script/Engine.PlayerStart"))
  (set `self.SpawnPoints` _outactors)
  (if (`KismetTextLibrary.EqualEqual_TextText` Team (`self.TeamA`))
    (bind _returnvalue (`|SpawnActorFromClass` Character (`self.GetTransform` (`|GetArrayItem` (`self.SpawnPoints`))) "Undefined" "OverrideRootScale" null null))
    (`Controller.Possess` PlayerController _returnvalue)
    (elif (`KismetTextLibrary.EqualEqual_TextText` Team (`self.TeamB`))
      (bind _returnvalue_2 (`|SpawnActorFromClass` Character (`self.GetTransform` (`|GetArrayItem` (`self.SpawnPoints`) 1)) "Undefined" "OverrideRootScale" null null))
      (`Controller.Possess` PlayerController _returnvalue_2))))

(fn `UserConstructionScript`)